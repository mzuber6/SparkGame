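; Player-controllable bike that drives, steers and leans through simple kinematic movement, with an orbitable spring-arm camera.
; Throttle and steer axes interpolate speed and steering angle, with a separate limit for reverse.
; Tick moves the actor forward with a swept offset, deriving yaw and lean from speed and angle, doubling turn rate in reverse.
; It also feeds speed and steering, damped at higher speed, to the BikeAnimation instance.
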(event EventBeginPlay
  (bind _asbike_animation (Utilities|Casting|CastToBikeAnimation (Components|SkeletalMesh|GetAnimInstance (Variables|Default|GetBike))))
  (Variables|Default|SetAnimInstance _asbike_animation))

(event EventTick
  (params (DeltaSeconds :type Float%20%28single-precision%29))
  (bind _animinstance (Variables|Default|GetAnimInstance))
  (bind _currentspeed (Variables|Default|GetCurrentSpeed))
  (Transformation|AddActorWorldOffset (* DeltaSeconds (* (Transformation|GetActorForwardVector) _currentspeed)) true)
  (Transformation|SetActorRelativeRotation (Math|Rotator|MakeRotator (Math|Interpolation|FInterpTo (Variables|Default|GetCurrentLeanAngle) (* (Variables|Default|GetCurrentAngle) (/ (Variables|Default|GetCurrentSpeed) (Variables|Default|GetMaxSpeed))) (Utilities|Time|GetWorldDeltaSeconds) 0.0) 0.0 (+ (.yaw (Transformation|GetActorRotation)) (* _currentspeed (Variables|Default|GetCurrentAngle) (Variables|Default|GetSpeedToRotationFactor) (Utilities|Time|GetWorldDeltaSeconds) (select (< _currentspeed 0.0) 2.0 1.0)))))
  (Variables|Default|SetCurrentLeanAngle (Math|Interpolation|FInterpTo (Variables|Default|GetCurrentLeanAngle) (* (Variables|Default|GetCurrentAngle) (/ (Variables|Default|GetCurrentSpeed) (Variables|Default|GetMaxSpeed))) (Utilities|Time|GetWorldDeltaSeconds) 0.0))
  (Variables|/Game/Bike/BikeAnimation.BikeAnimation_C|SetSpeed _animinstance (Variables|Default|GetCurrentSpeed))
  (Variables|/Game/Bike/BikeAnimation.BikeAnimation_C|SetSteering _animinstance (* (Variables|Default|GetCurrentAngle) (Math|Float|MapRangeClamped (Variables|Default|GetCurrentSpeed) 0.0 (Variables|Default|GetMaxSpeed) 1.0 0.2))))

(event Input|AxisEvents|InputAxisThrottle
  (params (AxisValue :type Float%20%28single-precision%29))
  (Variables|Default|SetCurrentSpeed (Math|Interpolation|FInterpTo (Variables|Default|GetCurrentSpeed) (* AxisValue (select (< AxisValue 0.0) (Variables|Default|GetMaxReverseSpeed) (Variables|Default|GetMaxSpeed))) (Utilities|Time|GetWorldDeltaSeconds) 1.0)))

(event Input|AxisEvents|InputAxisSteer
  (params (AxisValue :type Float%20%28single-precision%29))
  (Variables|Default|SetCurrentAngle (Math|Interpolation|FInterpTo (Variables|Default|GetCurrentAngle) (* AxisValue (Variables|Default|GetMaxSteeringAngle)) (Utilities|Time|GetWorldDeltaSeconds) 4.0)))

(event Input|AxisEvents|InputAxisLookRight
  (params (AxisValue :type Float%20%28single-precision%29))
  (Transformation|AddRelativeRotation (Variables|Default|GetSpringArm) (Math|Rotator|MakeRotator 0.0 0.0 AxisValue) false false))

(event Input|AxisEvents|InputAxisLookUp
  (params (AxisValue :type Float%20%28single-precision%29))
  (Transformation|AddRelativeRotation (Variables|Default|GetSpringArm) (Math|Rotator|MakeRotator 0.0 AxisValue 0.0) false false))

(fn ConstructionScript)